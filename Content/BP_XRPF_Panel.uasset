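; World actor hosting the XR privacy framework consent panel, covering hardware, location, social, spatial and biometric data categories.
; On BeginPlay it creates the privacy framework, passes per-category required flags to its UMG_XRPF_Panel widget and destroys itself on confirm.
; Debug functions simulate confirm and category toggles on the widget.
; Toggles act only on non-required categories, except location, whose check is inverted and toggles only when required.
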(event Custom|Destroy
  (Actor|DestroyActor))

(event EventBeginPlay
  (Class|XRPrivacyFrameworkBlueprints|CreatePrivacyFramework)
  (bind _asumg_xrpf_panel (Utilities|Casting|CastToUMG_XRPF_Panel (UserInterface|GetWidget (Variables|Default|GetWidget))))
  (Default|SetupRequirements _asumg_xrpf_panel (Variables|Default|GetIsHardwareDataRequired) (Variables|Default|GetIsLocationDataRequired) (Variables|Default|GetIsSocialDataRequired) (Variables|Default|GetIsSpatialDataRequired) (Variables|Default|GetIsBiometricDataRequired))
  (EventDispatchers|BindEventtoOnConfirmClick _asumg_xrpf_panel (delegate Custom|Destroy)))

(event Collision|EventActorBeginOverlap
  (params (OtherActor :type Actor%20Object%20Reference)))

(event EventEndPlay
  (params (EndPlayReason :type EEndPlayReason%20Enum :default "Destroyed")))

(fn ConstructionScript)

(fn DEBUGCONFIRM
  (bind _asumg_xrpf_panel (Utilities|Casting|CastToUMG_XRPF_Panel (UserInterface|GetWidget (Variables|Default|GetWidget))))
  (Default|ConfirmClicked _asumg_xrpf_panel))

(fn DEBUGHARDWARE
  (if (not (Variables|Default|GetIsHardwareDataRequired))
    (bind _asumg_xrpf_panel (Utilities|Casting|CastToUMG_XRPF_Panel (UserInterface|GetWidget (Variables|Default|GetWidget))))
    (Default|TOGGLEHARDWARE _asumg_xrpf_panel)))

(fn DEBUGLOC
  (if (Variables|Default|GetIsLocationDataRequired)
    (bind _asumg_xrpf_panel (Utilities|Casting|CastToUMG_XRPF_Panel (UserInterface|GetWidget (Variables|Default|GetWidget))))
    (Default|TOGGLELOCATION _asumg_xrpf_panel)))

(fn DEBUGSOCIAL
  (if (not (Variables|Default|GetIsSocialDataRequired))
    (bind _asumg_xrpf_panel (Utilities|Casting|CastToUMG_XRPF_Panel (UserInterface|GetWidget (Variables|Default|GetWidget))))
    (Default|TOGGLESOCIAL _asumg_xrpf_panel)))

(fn DEBUGSPATIAL
  (if (not (Variables|Default|GetIsSpatialDataRequired))
    (bind _asumg_xrpf_panel (Utilities|Casting|CastToUMG_XRPF_Panel (UserInterface|GetWidget (Variables|Default|GetWidget))))
    (Default|TOGGLESPATIAL _asumg_xrpf_panel)))

(fn DEBUGBIO
  (if (not (Variables|Default|GetIsBiometricDataRequired))
    (bind _asumg_xrpf_panel (Utilities|Casting|CastToUMG_XRPF_Panel (UserInterface|GetWidget (Variables|Default|GetWidget))))
    (Default|TOGGLEBIO _asumg_xrpf_panel)))